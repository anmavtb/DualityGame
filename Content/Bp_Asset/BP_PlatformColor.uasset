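; BP_PlatformColor is a two-color platform that is solid only while the player character's color state matches its own.
; The construction script picks one of two cube materials from the IsColor1 flag.
; BeginPlay caches the BP_Character instance, and Tick compares both IsColor1 flags every frame to switch the cube's collision on or off.
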(event `self.ReceiveBeginPlay`
  (bind _returnvalue (`GameplayStatics.GetActorOfClass` "/Game/PlayerCharacter/BP_Character.BP_Character_C"))
  (set `self.player` _returnvalue))

(event `self.ReceiveTick`
  (params (DeltaSeconds :type "Float (single-precision)"))
  (bind _cube (`self.Cube`))
  (if (== (`self.isColor1`) (`/Game/PlayerCharacter/BP_Character.isColor1` (`self.player`)))
    (`PrimitiveComponent.SetCollisionEnabled` _cube "QueryAndPhysics")
    (else
      (`PrimitiveComponent.SetCollisionEnabled` _cube "NoCollision"))))

(fn `UserConstructionScript`
  (bind _cube (`self.Cube`))
  (if (`self.isColor1`)
    (`PrimitiveComponent.SetMaterial` _cube 0 "/Game/Materials/MAT_Color1.MAT_Color1")
    (else
      (`PrimitiveComponent.SetMaterial` _cube 0 "/Game/Materials/MAT_Color2.MAT_Color2"))))