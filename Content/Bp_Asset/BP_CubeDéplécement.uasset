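; BP_CubeDéplacement is a movable cube that toggles physics and collision based on the state of the player's BP_Character.
; Tick disables the cube's collision while the player's IsColor1 flag is true and restores query-and-physics collision otherwise.
; The AxeX overlap volume enables physics simulation on the cube and sets the character's Move flag when the character enters, then clears both on exit.
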(event `self.ReceiveBeginPlay`
  (bind _returnvalue (`GameplayStatics.GetActorOfClass` "/Game/PlayerCharacter/BP_Character.BP_Character_C"))
  (set `self.player` _returnvalue))

(event `self.ReceiveTick`
  (params (DeltaSeconds :type "Float (single-precision)"))
  (bind _cubemove (`self.CubeMove`))
  (if (`/Game/PlayerCharacter/BP_Character.isColor1` (`self.player`))
    (`PrimitiveComponent.SetCollisionEnabled` _cubemove "NoCollision")
    (else
      (`PrimitiveComponent.SetCollisionEnabled` _cubemove "QueryAndPhysics"))))

(event `self.Axe X.OnComponentBeginOverlap`
  (params (OverlappedComponent :type "PrimitiveComponent Object Reference") (OtherActor :type "Actor Object Reference") (OtherComp :type "PrimitiveComponent Object Reference") (OtherBodyIndex :type Integer) (bFromSweep :type Boolean) (SweepResult :type "HitResult Structure (by ref)"))
  ;[1 1 1] Axe X Simulate Physics
  (bind _asbp_character (cast `/Game/PlayerCharacter/BP_Character` OtherActor))
  (`PrimitiveComponent.SetSimulatePhysics` (`self.CubeMove`) true)
  (set `/Game/PlayerCharacter/BP_Character.Move?` true _asbp_character))

(event `self.Axe X.OnComponentEndOverlap`
  (params (OverlappedComponent :type "PrimitiveComponent Object Reference") (OtherActor :type "Actor Object Reference") (OtherComp :type "PrimitiveComponent Object Reference") (OtherBodyIndex :type Integer))
  ;[1 1 1] Axe X Simulate Physics
  (bind _asbp_character (cast `/Game/PlayerCharacter/BP_Character` OtherActor))
  (`PrimitiveComponent.SetSimulatePhysics` (`self.CubeMove`) false)
  (set `/Game/PlayerCharacter/BP_Character.Move?` false _asbp_character))

(fn `UserConstructionScript`)